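; Conflict mode ruleset that sets up and drives the resource economy through a quartermaster actor.
; On BeginPlay it spawns BP_Conflict_Quartermaster as an owned actor and publishes the reference to BP_GameMode_Conflict.
; A looping ten-second timer calls the quartermaster's resource tick.
; The VehicleDestroyed event only prints a debug message.
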(event EventBeginPlay
  (bind _returnvalue (Game|SpawnActorfromClass "/SIC/Gameplay/GameModes/Conflict/BP_Conflict_Quartermaster.BP_Conflict_Quartermaster_C" (Math|Transform|MakeTransform "0, 0, 0") "AlwaysSpawn" self 0))
  (bind _output_get (Variables|Default|SetQuartermaster _returnvalue))
  (Utilities|Time|SetTimerbyFunctionName 0 "ResourceTimerFunc" 1e+01 true)
  (bind _asbp_game_mode_conflict (Utilities|Casting|CastToBP_GameMode_Conflict (CallFunction|GetSquadGameMode)))
  (Variables|/SIC/Gameplay/GameModes/BP_GameMode_Conflict.BP_GameMode_Conflict_C|SetQuarterMasterRef _asbp_game_mode_conflict _output_get)
  (Development|PrintString "Successfully set QM reference"))

(event Collision|EventActorBeginOverlap
  (params (OtherActor :type Actor%20Object%20Reference)))

(event EventTick
  (params (DeltaSeconds :type Float%20%28single-precision%29)))

(event EventVehicleDestroyed
  (params (Killer :type SQ%20Player%20Controller%20Object%20Reference) (Victim :type SQ%20Player%20Controller%20Object%20Reference) (DestroyedVehicle :type SQ%20Vehicle%20Object%20Reference))
  (Development|PrintString "Vehicle Destroyed"))

(fn ConstructionScript)

(fn ResourceTimerFunc
  (Default|AddResourcesTick (Variables|Default|GetQuartermaster)))