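; Team vehicle depot actor for the Conflict game mode that spawns a random vehicle from its list when a soldier overlaps it.
; Cost derives from the vehicle's destruction ticket loss in the kill/death ruleset's Team One settings, whichever team owns the depot.
; The quartermaster charges DepotTeam's resources; on success the vehicle spawns at VehicleSpawn for that team.
; The quartermaster's result message is printed, and BeginPlay labels the depot with its team name.
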(event EventBeginPlay
  (CallFunction|RenderTeamInfo))

(event Collision|EventActorBeginOverlap
  (params (OtherActor :type Actor%20Object%20Reference))
  (bind _spawnablevehicles (Variables|Default|GetSpawnableVehicles))
  (Utilities|Casting|CastToSQSoldier OtherActor)
  (CallFunction|SpawnVehicle (Utilities|Array|Get(acopy) _spawnablevehicles (Math|Random|RandomIntegerinRange 0 (- (Utilities|Array|Length _spawnablevehicles) 1)))))

(event EventTick
  (params (DeltaSeconds :type Float%20%28single-precision%29)))

(fn ConstructionScript)

(fn SpawnVehicle
  (params (VehicleType :type SQ%20Vehicle%20Class%20Reference))
  (bind _asbp_game_mode_conflict (Utilities|Casting|CastToBP_GameMode_Conflict (CallFunction|GetSquadGameMode)))
  (for _array_element (Variables|/Script/Squad.SQGameMode|GetRuleSetClasses _asbp_game_mode_conflict)
    (bind _asbp_kill_death_ruleset (Utilities|Casting|CastToBP_KillDeathRulesetClass _array_element))
    (for _array_element_2 (.VehicleSettings (Utilities|Struct|BreakSQKillDeathSettings (.TeamOneSettings (Utilities|GetClassDefaults _asbp_kill_death_ruleset))))
      (if (== (.VehicleType (Utilities|Struct|BreakSQVehicleDeathTicket _array_element_2)) VehicleType)
        (bind _output_get (LocalVariables|SetVehicleSpawnCost (* (.TicketsLostOnVehicleDestroy (Utilities|Struct|BreakSQVehicleDeathTicket _array_element_2)) 100)))
        (bind (_success _message) (Default|ConsumeTeamResources (Variables|/SIC/Gameplay/GameModes/BP_GameMode_Conflict.BP_GameMode_Conflict_C|GetQuarterMasterRef _asbp_game_mode_conflict) (Variables|Default|GetDepotTeam) (LocalVariables|GetVehicleSpawnCost)))
        (if _success
          (Game|SpawnActorfromClass VehicleType (Transformation|GetWorldTransform (Variables|Default|GetVehicleSpawn)) "AlwaysSpawn" 0 (Variables|Default|GetDepotTeam) 0))
        (Development|PrintString _message)))))

(fn RenderTeamInfo
  (Rendering|Components|TextRender|SetText (Variables|Default|GetTeamName) (Utilities|Text|ToText(String) (Utilities|String|Append (Variables|/Script/Squad.SQTeamInfo|GetName (CallFunction|GetTeamInfobyId (Math|Conversions|ToInteger(Byte) (Variables|Default|GetDepotTeam)))) " Vehicle Spawn Depot"))))