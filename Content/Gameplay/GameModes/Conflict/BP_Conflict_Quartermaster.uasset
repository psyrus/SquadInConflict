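; Quartermaster for the Conflict game mode that keeps the resource pools for two teams and their squads.
; AddResourcesTick, not called within this Blueprint, grows team pools by base rate times modifier and squad pools by player count across fireteams.
; Squads come from the Squad game mode and join a per-squad map on first tick.
; ConsumeTeamResources deducts affordable costs and returns a status message; squad spending is an empty stub.
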(event EventBeginPlay
  (Development|PrintString "Quartermaster initialized!"))

(event Collision|EventActorBeginOverlap
  (params (OtherActor :type Actor%20Object%20Reference)))

(event EventTick
  (params (DeltaSeconds :type Float%20%28single-precision%29)))

(fn ConstructionScript
  (bind _teamresources (Variables|Default|GetTeamResources))
  (Utilities|Array|Add _teamresources (Utilities|Struct|MakeConflictTeamResources "Team_Neutral" 0 300 1.0))
  (Utilities|Array|Add _teamresources (Utilities|Struct|MakeConflictTeamResources "Team_Neutral" 0 300 1.0)))

(fn AddResourcesTick
  (Development|PrintString "Resources Ticked!")
  (CallFunction|AddTeamResourcesTick)
  (CallFunction|AddSquadsResourcesTick))

(fn AddTeamResourcesTick
  (for (_array_element _array_index) (Variables|Default|GetTeamResources)
    (Utilities|Array|SetArrayElem (Variables|Default|GetTeamResources) _array_index (Utilities|Struct|MakeConflictTeamResources (.TeamEnum (Utilities|Struct|BreakConflictTeamResources _array_element)) (+ (.CurrentTeamResources (Utilities|Struct|BreakConflictTeamResources _array_element)) (Math|Float|Round (* (.BaseResourceRate (Utilities|Struct|BreakConflictTeamResources _array_element)) (.CurrentRateModifier (Utilities|Struct|BreakConflictTeamResources _array_element))))) (.BaseResourceRate (Utilities|Struct|BreakConflictTeamResources _array_element)) (.CurrentRateModifier (Utilities|Struct|BreakConflictTeamResources _array_element))))
    (Development|PrintString (Utilities|String|Append "Team " (Utilities|String|ToString(Integer) _array_index) " has " (Utilities|String|ToString(Integer) (.CurrentTeamResources (Utilities|Struct|BreakConflictTeamResources _array_element))) " resources"))))

(fn AddSquadsResourcesTick
  (for _array_element (Variables|/Script/Squad.SQGameMode|GetIndexedTeams (CallFunction|GetSquadGameMode))
    (for _array_element_2 (Variables|/Script/Squad.SQTeam|GetSquads _array_element)
      (LocalVariables|SetCurrentSquad _array_element_2)
      (if (.ReturnValue (Utilities|Map|Find (Variables|Default|GetSquadResources) (LocalVariables|GetCurrentSquad)))
        _
        (else
          (Utilities|Map|Add (Variables|Default|GetSquadResources) (LocalVariables|GetCurrentSquad) (Utilities|Struct|MakeConflictSquadResources))
          (Development|PrintString "Added Squad to Dictionary")))
      (for _array_element_3 (Variables|/Script/Squad.SQSquad|GetFireTeams (LocalVariables|GetCurrentSquad))
        (Utilities|Map|Add (Variables|Default|GetSquadResources) (LocalVariables|GetCurrentSquad) (Utilities|Struct|MakeConflictSquadResources (+ (* (Utilities|Array|Length (Utilities|Struct|BreakSQFireTeam _array_element_3)) (Variables|Default|GetPerPlayerResourceGainRate)) (Utilities|Struct|BreakConflictSquadResources (.Value (Utilities|Map|Find (Variables|Default|GetSquadResources) (LocalVariables|GetCurrentSquad))))))))
      ;[1 1 1] Debug Squad Points
      (Development|PrintString (Utilities|String|Append "Squad (" (Variables|/Script/Squad.SQSquadState|GetName (Variables|/Script/Squad.SQSquad|GetSquadState (LocalVariables|GetCurrentSquad))) ") has [" (Utilities|String|ToString(Integer) (Utilities|Struct|BreakConflictSquadResources (.Value (Utilities|Map|Find (Variables|Default|GetSquadResources) (LocalVariables|GetCurrentSquad))))) "] points available")))))

(fn ConsumeSquadResources)

(fn ConsumeTeamResources
  (params (ConsumingTeam :type ESQTeam%20Enum) (AmountToConsume :type Integer))
  (bind _returnvalue (Math|Conversions|ToInteger(Byte) ConsumingTeam))
  (bind _teamresources (Variables|Default|GetTeamResources))
  (bind _returnvalue_2 (Math|Conversions|ToInteger(Byte) ConsumingTeam))
  (bind _output (Utilities|Array|Get(acopy) _teamresources _returnvalue))
  (bind (_teamenum _currentteamresources _baseresourcerate _currentratemodifier) (Utilities|Struct|BreakConflictTeamResources _output))
  (bind _returnvalue_3 (>= _currentteamresources AmountToConsume))
  (bind _output_get (LocalVariables|SetCurrentResources _currentteamresources))
  (if _returnvalue_3
    (Utilities|Array|SetArrayElem (Variables|Default|GetTeamResources) _returnvalue_2 (Utilities|Struct|MakeConflictTeamResources _teamenum (- _output_get AmountToConsume) _baseresourcerate _currentratemodifier))
    (LocalVariables|SetMessageToReturn (Utilities|String|Append "Deducted " (Utilities|String|ToString(Integer) AmountToConsume) " resources from team " (Utilities|String|ToString(Integer) _returnvalue_2) ". Remaining Resources: " (Utilities|String|ToString(Integer) (- _output_get AmountToConsume))))
    (else
      (LocalVariables|SetMessageToReturn "Insufficient Resources")))
  (return _returnvalue_3 (LocalVariables|GetMessageToReturn)))